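; Door Blueprint meant to swing open in a direction chosen by the player's side and close again.
; IsForward tests whether the angle between the player-to-door vector and the door's forward vector is under 90 degrees, selecting one of two rotation timelines.
; DoorState and a WaitForOpen flag handle reversing a swing and reopening after closing.
; Both open and close chains have no connected trigger, so the logic never runs as wired.
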(fn ConstructionScript)

(fn AngleBetween2Vectors
  (params (Vector1 :type Vector) (Vector2 :type Vector))
  (return (Math|Trig|RadiansToDegrees (Math|Trig|Acos(Degrees) (Math|Vector|DotProduct (Math|Vector|Normalize Vector1) (Math|Vector|Normalize Vector2))))))

(fn IsForward
  (bind _angle (CallFunction|AngleBetween2Vectors (- (Transformation|GetWorldLocation (Variables|Default|GetDoorRoot)) (Transformation|GetActorLocation (Game|GetPlayerCharacter 0))) (Math|Vector|GetForwardVector (Variables|Default|GetDoorRoot))))
  (return (< _angle 9e+01)))