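; Elevator doors that characters open by filling a progress slider, shown while they are inside the trigger and the doors are still closed.
; Overlap hands Opening and Closing to each BP_Character, and leaving unbinds them and starts Closing.
; Opening and Closing raise or drain a value through next-tick delay loops, updating every slider in range.
; At full, a timeline lerps both doors to their open markers permanently.
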(event OnComponentBeginOverlap(All)
  (params (OverlappedComponent :type Primitive%20Component%20Object%20Reference) (OtherActor :type Actor%20Object%20Reference) (OtherComp :type Primitive%20Component%20Object%20Reference) (OtherBodyIndex :type Integer) (bFromSweep :type Boolean) (SweepResult :type Hit%20Result%20Structure%20%28by%20ref%29))
  (bind _asbp_character (Utilities|Casting|CastToBP_Character OtherActor))
  (if (not (Variables|Default|GetIsOpened))
    (Default|ShowSlider _asbp_character)
    (Default|SetSliderValue _asbp_character (Variables|Default|GetValue))
    (Utilities|Array|Add (Variables|Default|GetCharactersInRange) _asbp_character)
    (EventDispatchers|AssignOpening _asbp_character (delegate Custom|Opening))
    (EventDispatchers|BindEventtoClosing _asbp_character (delegate Custom|Closing))))

(event OnComponentEndOverlap(All)
  (params (OverlappedComponent :type Primitive%20Component%20Object%20Reference) (OtherActor :type Actor%20Object%20Reference) (OtherComp :type Primitive%20Component%20Object%20Reference) (OtherBodyIndex :type Integer))
  (bind _charactersinrange (Variables|Default|GetCharactersInRange))
  (bind _asbp_character (Utilities|Casting|CastToBP_Character OtherActor))
  (if (not (Variables|Default|GetIsOpened))
    (if (Utilities|Array|ContainsItem _charactersinrange _asbp_character)
      (Default|HideSlider _asbp_character)
      (Utilities|Array|RemoveItem _charactersinrange _asbp_character)
      (EventDispatchers|UnbindEventfromOpening _asbp_character (delegate Custom|Opening))
      (EventDispatchers|UnbindEventfromClosing _asbp_character (delegate Custom|Closing))
      (CallFunction|Closing))))

(event Custom|Opening
  (if (Variables|Default|GetIsOpened)
    _
    (else
      _))
  (Development|PrintString "Open")
  (Variables|Default|SetIsInProgress true)
  (if (Variables|Default|GetIsInProgress) :!label _label
    (bind (_output_get _success) (CallFunction|Increase (Variables|Default|GetValue)))
    (for _array_element (Variables|Default|GetCharactersInRange)
      (Default|SetSliderValue _array_element _output_get))
    (if _success
      (Utilities|FlowControl|DelayUntilNextTick)
      (goto _label)
      (else
        (CallFunction|Open)
        (Variables|Default|SetIsOpened true)
        (for _array_element_2 (Variables|Default|GetCharactersInRange)
          (Default|HideSlider _array_element_2)
          (EventDispatchers|UnbindEventfromOpening _array_element_2 (delegate Custom|Opening))
          (EventDispatchers|UnbindEventfromClosing _array_element_2 (delegate Custom|Closing)))))))

(event Custom|Closing
  (if (Variables|Default|GetIsOpened)
    _
    (else
      _))
  (Development|PrintString "Close")
  (Variables|Default|SetIsInProgress false)
  (if (not (Variables|Default|GetIsInProgress)) :!label _label
    (bind (_output_get _success) (CallFunction|Decrease (Variables|Default|GetValue)))
    (for _array_element (Variables|Default|GetCharactersInRange)
      (Default|SetSliderValue _array_element _output_get))
    (if _success
      (Utilities|FlowControl|DelayUntilNextTick)
      (goto _label))))

(event Custom|Open
  (bind _angle (Timeline|OpenTimeline Play)
    (:Update
      (Utilities|FlowControl|Sequence
        (:then_0
          (Transformation|SetWorldLocation (Variables|Default|GetLeft) (Math|Vector|Lerp(Vector) (Transformation|GetWorldLocation (Variables|Default|GetDoorLeftClosed)) (Transformation|GetWorldLocation (Variables|Default|GetDoorLeftOpened)) _angle) false false))
        (:then_1
          (Transformation|SetWorldLocation (Variables|Default|GetRight) (Math|Vector|Lerp(Vector) (Transformation|GetWorldLocation (Variables|Default|GetDoorRightClosed)) (Transformation|GetWorldLocation (Variables|Default|GetDoorRightOpened)) _angle) false false))))))

(fn ConstructionScript)

(fn AngleBetween2Vectors
  (params (Vector1 :type Vector) (Vector2 :type Vector))
  (return (Math|Trig|RadiansToDegrees (Math|Trig|Acos(Degrees) (Math|Vector|DotProduct (Math|Vector|Normalize Vector1) (Math|Vector|Normalize Vector2))))))

(fn IsForward
  (bind _angle (CallFunction|AngleBetween2Vectors (- (Transformation|GetWorldLocation (Variables|Default|GetDoorRoot)) (Transformation|GetActorLocation (Game|GetPlayerCharacter 0))) (Math|Vector|GetForwardVector (Variables|Default|GetDoorRoot))))
  (return (< _angle 9e+01)))

(fn Increase
  (params (Value :type Float%20%28double-precision%29))
  (bind _returnvalue (< Value 1.0))
  (if _returnvalue
    (Variables|Default|SetValue (+ Value (* (Utilities|Time|GetWorldDeltaSeconds) 0.5)))
    (else
      (Variables|Default|SetValue 1.0)))
  (return Value _returnvalue))

(fn Decrease
  (params (Value :type Float%20%28double-precision%29))
  (bind _returnvalue (< 0.0 Value))
  (if _returnvalue
    (bind _output_get (Variables|Default|SetValue (- (Variables|Default|GetValue) (* (Utilities|Time|GetWorldDeltaSeconds) 0.5))))
    (else
      (Variables|Default|SetValue 0.0)))
  (return _output_get _returnvalue))